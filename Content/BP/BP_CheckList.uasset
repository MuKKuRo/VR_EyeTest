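; BP_CheckList is a checklist Blueprint that publishes the world positions of its text slots to the game instance.
; On BeginPlay it reads locations from numbered components, grouped into one single position and four arrays of two, three, four and four entries.
; It casts the game instance to Main_Instance and copies each group into the matching TextLoc variable there.
; Component 55 is left out of the last group.
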(event `self.ReceiveBeginPlay`
  (bind _output_get (set `self.TextLoc_1` (`SceneComponent.K2_GetComponentLocation` (`self.1-1`))))
  (bind _output_get_2 (set `self.TextLoc_2` (`|MakeArray` (`SceneComponent.K2_GetComponentLocation` (`self.2-1`)) (`SceneComponent.K2_GetComponentLocation` (`self.2-2`)))))
  (bind _output_get_3 (set `self.TextLoc_3` (`|MakeArray` (`SceneComponent.K2_GetComponentLocation` (`self.3-1`)) (`SceneComponent.K2_GetComponentLocation` (`self.3-2`)) (`SceneComponent.K2_GetComponentLocation` (`self.3-3`)))))
  (bind _output_get_4 (set `self.TextLoc_4` (`|MakeArray` (`SceneComponent.K2_GetComponentLocation` (`self.4-1`)) (`SceneComponent.K2_GetComponentLocation` (`self.4-2`)) (`SceneComponent.K2_GetComponentLocation` (`self.4-3`)) (`SceneComponent.K2_GetComponentLocation` (`self.4-4`)))))
  (bind _output_get_5 (set `self.TextLoc_5` (`|MakeArray` (`SceneComponent.K2_GetComponentLocation` (`self.5-1`)) (`SceneComponent.K2_GetComponentLocation` (`self.5-2`)) (`SceneComponent.K2_GetComponentLocation` (`self.5-3`)) (`SceneComponent.K2_GetComponentLocation` (`self.5-4`)))))
  (bind _asmain_instance (cast `/Game/Basic_Moduls/Main_Instance` (`GameplayStatics.GetGameInstance`)))
  (set `/Game/Basic_Moduls/Main_Instance.Text_Loc1_ins` _output_get _asmain_instance)
  (set `/Game/Basic_Moduls/Main_Instance.Text_Loc2_ins` _output_get_2 _asmain_instance)
  (set `/Game/Basic_Moduls/Main_Instance.Text_Loc3_ins` _output_get_3 _asmain_instance)
  (set `/Game/Basic_Moduls/Main_Instance.Text_Loc4_ins` _output_get_4 _asmain_instance)
  (set `/Game/Basic_Moduls/Main_Instance.Text_Loc5_ins` _output_get_5 _asmain_instance))

(fn `UserConstructionScript`)