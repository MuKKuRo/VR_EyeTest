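; BP_Pointer is an eye test Blueprint that simulates an instructor's laser pointer with a debug line trace.
; BeginPlay fires the test start event three times at five-second intervals, printing a message each time.
; Each event traces on Visibility from the Instructor component to a text location stored in Main_Instance, drawing the line briefly.
; The Point Random Elim function is empty, and a random array pick is left unused.
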(event `self.ReceiveBeginPlay`
  (`KismetSystemLibrary.Delay` 5.0)
  (`KismetSystemLibrary.PrintString` "Laser pointing")
  (`self.Ev_Test Start`)
  (`KismetSystemLibrary.Delay` 5.0)
  (`KismetSystemLibrary.PrintString` "Laser pointing")
  (`self.Ev_Test Start`)
  (`KismetSystemLibrary.Delay` 5.0)
  (`KismetSystemLibrary.PrintString` "Laser pointing")
  (`self.Ev_Test Start`))

(event `Ev_Test Start`
  (bind _asmain_instance (cast `/Game/Basic_Moduls/Main_Instance` (`GameplayStatics.GetGameInstance`)))
  (`KismetSystemLibrary.LineTraceSingle` :`Start` (`SceneComponent.K2_GetComponentLocation` (`self.Instructor`)) :`End` (`/Game/Basic_Moduls/Main_Instance.Text_Loc1_ins` _asmain_instance) :`TraceChannel` "TraceTypeQuery1" :`DrawDebugType` "ForDuration" :`DrawTime` 3.0))

(fn `Point Random Elim`
  (params (`Text Array` :type "Array of Vector Structure")))

(fn `UserConstructionScript`)