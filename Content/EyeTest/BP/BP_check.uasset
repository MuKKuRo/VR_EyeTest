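; BP_check is an eye test Blueprint that reveals random letters from three hard-coded rows and tallies answers.
; On BeginPlay it fills the arrays, then runs SetVisibility and TestProcess on each row in immediate succession.
; SetVisibility reveals letters through a "Text visibility" material parameter.
; TestProcess checks first-row letter tags and AnswerCorrect, updates PlayerState counters, and either reveals another letter, stops, or disables input after repeated errors.
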(event `self.ReceiveBeginPlay`
  (`self.Set Text Array`)
  (bind _output_array (`self.Set Visibility` (`self.Array_01`)))
  (`self.Test Process` _output_array)
  (`KismetSystemLibrary.PrintString` "arra")
  (bind _output_array_2 (`self.Set Visibility` (`self.Array_02`)))
  (`self.Test Process` _output_array_2)
  (bind _output_array_3 (`self.Set Visibility` (`self.Array_03`)))
  (`self.Test Process` _output_array_3))

(fn `Set Text Array`
  (set `self.Array_01` (`|MakeArray` (`self.1-1T`) (`self.1-2Z`) (`self.1-3C`) (`self.1-4O`)))
  (set `self.Array_02` (`|MakeArray` (`self.2-1L`) (`self.2-2D`) (`self.2-3P`) (`self.2-4O`) (`self.2-5F`)))
  (set `self.Array_03` (`|MakeArray` (`self.3-1P`) (`self.3-2T`) (`self.3-3O`) (`self.3-4C`) (`self.3-5E`)))
  (return))

(fn `Set Visibility`
  (params (`input array` :type "Array of StaticMeshComponent Object Reference"))
  (returns (`output array` :type "Array of StaticMeshComponent Object Reference"))
  (`MeshComponent.SetScalarParameterValueOnMaterials` (`|GetArrayItem` `input array` (`KismetMathLibrary.RandomIntegerInRange` 0 (`KismetArrayLibrary.Array_Length` `input array`))) "Text visibility" 1.0)
  (`KismetSystemLibrary.PrintString` "text_Set successfully")
  (return `input array`))

(fn `Test Process`
  (params (`input array` :type "Array of StaticMeshComponent Object Reference"))
  (if (and (or (`self.ActorHasTag` "T") (`self.ActorHasTag` "Z") (`self.ActorHasTag` "C") (`self.ActorHasTag` "O")) (`self.answer correct?`))
    (bind _result (`/Engine/EditorBlueprintResources/StandardMacros.IncrementInt` (`/Game/EyeTest/Basic_Moduls/BP_UserState.Correct Count` (`self.PlayerState`)))
      (:`  `
        (if (>= _result (/ (`KismetArrayLibrary.Array_Length` `input array`) 2))
          (return)
          (else
            (`self.Set Visibility` `input array`)))))
    (else
      (bind _result_2 (`/Engine/EditorBlueprintResources/StandardMacros.IncrementInt` (`/Game/EyeTest/Basic_Moduls/BP_UserState.Incorrect Count` (`self.PlayerState`)))
        (:`  `
          (if (>= _result_2 3)
            (`self.DisableInput` (`PlayerState.GetPlayerController` (`self.PlayerState`)) null)
            (else
              (`self.Set Visibility` `input array`))))))))

(fn `UserConstructionScript`)