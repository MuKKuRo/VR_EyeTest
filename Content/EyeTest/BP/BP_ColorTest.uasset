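; BP_ColorTest is an eye-test Blueprint that shows a timed sequence of ten color test components, one at a time.
; BeginPlay builds the component array, shows the entry at CurrentIndex and starts a looping five-second timer.
; Each timer tick increments CurrentIndex and calls SetVisibility, which hides every element and then reveals the current one.
; The index has no wrap or bounds check, so it keeps counting past the last element.
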(event `self.ReceiveBeginPlay`
  (bind _output_get (`self.Array`))
  (`KismetSystemLibrary.K2_SetTimerDelegate` (delegate `EyeTest`) 5.0 true)
  (`self.Set Visibility` _output_get))

(event `EyeTest`
  (`/Engine/EditorBlueprintResources/StandardMacros.IncrementInt` (`self.CurrentIndex`)
    (:`  `
      (`self.Set Visibility` (`self.EyeTestArray`)))))

(fn `Array`
  (returns (Output_Get :type "Array of StaticMeshComponent Object Reference"))
  (bind _output_get (set `self.EyeTestArray` (`|MakeArray` (`self.ColorTest01`) (`self.ColorTest02`) (`self.ColorTest03`) (`self.ColorTest04`) (`self.ColorTest05`) (`self.ColorTest06`) (`self.ColorTest07`) (`self.ColorTest08`) (`self.ColorTest09`) (`self.ColorTest10`))))
  (return _output_get))

(fn `Set Visibility`
  (params (Array :type "Array of StaticMeshComponent Object Reference"))
  (for _array_element Array
    (`SceneComponent.SetVisibility` _array_element false false))
  (`SceneComponent.SetVisibility` (`|GetArrayItem` Array (`self.CurrentIndex`)) true false))

(fn `UserConstructionScript`)